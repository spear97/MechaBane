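; Player character Blueprint for a shooter, handling movement, look, jump, sprint and a switchable rifle and launcher.
; Input sets the weapon enum, and Tick polls it to toggle weapon and player visibility and cancel aiming on the launcher.
; Rifle aiming shifts and zooms the camera.
; Fire sets a Firing flag and directly triggers only the launcher; separate events and functions spawn socketed projectiles with muzzle effects and sound.
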(event Custom|Aim_Rifle
  (bind _camera (Variables|Default|GetCamera))
  ;[1 1 1] Aiming for Rifle
  (Variables|Default|SetAiming true)
  (Transformation|SetRelativeLocation _camera "-22.277430,-12.747785,54.198795" false false)
  (Camera|SetFieldOfView _camera 38.457138))

(event Custom|Reset
  (bind _camera (Variables|Default|GetCamera))
  ;[1 1 1] Aiming for Rifle
  (Variables|Default|SetAiming false)
  (Transformation|SetRelativeLocation _camera "-22.277552,-14.043266,55.125637" false false)
  (Camera|SetFieldOfView _camera 9e+01))

(event Custom|Launcher%20Firing
  ;[1 1 1] Firing Functionality
  (Variables|Default|SetFiring true)
  (CallFunction|FireLauncher)
  (Utilities|FlowControl|Delay 0.29)
  (Variables|Default|SetFiring false))

(event Custom|Fire%20Rifle%20Projectile
  (bind _rifle (Variables|Default|GetRifle))
  (bind _returnvalue (Transformation|GetSocketTransform _rifle "MuzzleFlashSocket" "RTS_World"))
  (bind (_location _rotation _scale) (Math|Transform|BreakTransform _returnvalue))
  ;[1 1 1] Spawn Rifle Projectile
  (Game|SpawnActorfromClass "/Game/BluePrint/Rifle_Projectile.Rifle_Projectile_C" _returnvalue "Undefined" 0 0)
  (Effects|SpawnEmitteratLocation "/Game/SciFiWeapLight/FX/Particles/P_AssaultRifle_MuzzleFlash_Dark.P_AssaultRifle_MuzzleFlash_Dark" _location _rotation _scale)
  (Audio|PlaySoundatLocation "/Game/SciFiWeapLight/Sound/Rifle/Rifle_Fire_Cue.Rifle_Fire_Cue" _location "0, 0, 0" 1.0 1.0 0.0 0 0 0))

(event Custom|Fire%20Launcher%20Projectile
  (bind _launcher (Variables|Default|GetLauncher))
  (bind _returnvalue (Transformation|GetSocketTransform _launcher "MuzzleFlashSocket" "RTS_World"))
  (bind (_location _rotation _scale) (Math|Transform|BreakTransform _returnvalue))
  ;[1 1 1] Spawn Launcher Projectile
  (Game|SpawnActorfromClass "/Game/BluePrint/Launcher_Projectile.Launcher_Projectile_C" _returnvalue "Undefined" 0 0)
  (Effects|SpawnEmitteratLocation "/Game/Effects/ParticleSystems/Weapons/RocketLauncher/Muzzle/P_Launcher_MF.P_Launcher_MF" _location _rotation _scale)
  (Audio|PlaySoundatLocation "/Game/Sounds/Weapons/GrenadeLauncher/SCue_Launcher_Shoot.SCue_Launcher_Shoot" _location "0, 0, 0" 1.0 1.0 0.0 0 0 0))

(event EventTick
  (params (DeltaSeconds :type Float%20%28single-precision%29))
  (Utilities|FlowControl|Sequence
    (:then_0
      (CallFunction|SetRifle))
    (:then_1
      (CallFunction|SetLauncher))
    (:then_2
      (CallFunction|ResetADS))))

(event EventBeginPlay
  (Rendering|SetVisibility (Variables|Default|GetPlayer) false false))

(event Input|ActionEvents|InputActionJump
  (params (Key :type Key%20Structure :default "None"))
  ;[1 1 1] Jump Button
  (:Pressed
    (Character|Jump))
  (:Released
    (Character|StopJumping)))

(event Input|ActionEvents|InputActionSprint
  (params (Key :type Key%20Structure :default "None"))
  (:Pressed
    (CallFunction|Sprint))
  (:Released
    (CallFunction|StopSprint)))

(event Input|ActionEvents|InputActionAim
  (params (Key :type Key%20Structure :default "None"))
  ;[1 1 1] Call Aim Events dependent Upon the Selected Weapon
  (:Pressed
    (if (Utilities|Enum|Equal(Enum) (Variables|Default|GetWeaponList) "NewEnumerator0")
      (CallFunction|AimRifle)))
  (:Released
    (CallFunction|Reset)))

(event Input|ActionEvents|InputActionFire
  (params (Key :type Key%20Structure :default "None"))
  ;[1 1 1] Firing Functionality
  (:Pressed
    (Variables|Default|SetFiring true)
    (if (Utilities|Enum|Equal(Enum) (Variables|Default|GetWeaponList) "NewEnumerator1")
      (CallFunction|LauncherFiring)))
  (:Released
    (Variables|Default|SetFiring false)))

(event Input|ActionEvents|InputActionEquipRifle
  (params (Key :type Key%20Structure :default "None"))
  ;[1 1 1] Switch Between Weapons
  (:Pressed
    (if (not (Utilities|Enum|Equal(Enum) (Variables|Default|GetWeaponList) "NewEnumerator0"))
      (Variables|Default|SetWeaponList "NewEnumerator0"))))

(event Input|ActionEvents|InputActionEquipLauncher
  (params (Key :type Key%20Structure :default "None"))
  ;[1 1 1] Switch Between Weapons
  (:Pressed
    (if (not (Utilities|Enum|Equal(Enum) (Variables|Default|GetWeaponList) "NewEnumerator1"))
      (Variables|Default|SetWeaponList "NewEnumerator1"))))

(event Input|AxisEvents|InputAxisLookUp
  (params (AxisValue :type Float%20%28single-precision%29))
  ;[1 1 1] Rotation
  (Pawn|Input|AddControllerPitchInput AxisValue))

(event Input|AxisEvents|InputAxisTurn
  (params (AxisValue :type Float%20%28single-precision%29))
  ;[1 1 1] Rotation
  (Pawn|Input|AddControllerYawInput AxisValue))

(event Input|AxisEvents|InputAxisMoveForward
  (params (AxisValue :type Float%20%28single-precision%29))
  ;[1 1 1] Add Movement Input
  (Pawn|Input|AddMovementInput (Math|Vector|GetForwardVector (Variables|Default|GetCamera)) AxisValue false))

(event Input|AxisEvents|InputAxisMoveRight
  (params (AxisValue :type Float%20%28single-precision%29))
  ;[1 1 1] Add Movement Input
  (Pawn|Input|AddMovementInput (Math|Vector|GetRightVector (Variables|Default|GetCamera)) AxisValue false))

(fn ConstructionScript)

(fn SetRifle
  ;[1 1 1] Set Rifle Visibility if Weapon is Set to Rifle
  (if (Utilities|Enum|Equal(Enum) (Variables|Default|GetWeaponList) "NewEnumerator0")
    (Rendering|SetVisibility (Variables|Default|GetLauncher) false false)
    (Rendering|SetVisibility (Variables|Default|GetRifle) true false)
    (Rendering|SetVisibility (Variables|Default|GetLauncher_Player) false false)
    (Rendering|SetVisibility (Variables|Default|GetRifle_Player) true false)))

(fn SetLauncher
  ;[1 1 1] Set Launcher Visibility if Weapon is Set to Launcher
  (if (Utilities|Enum|Equal(Enum) (Variables|Default|GetWeaponList) "NewEnumerator1")
    (Rendering|SetVisibility (Variables|Default|GetRifle) false false)
    (Rendering|SetVisibility (Variables|Default|GetLauncher) true false)
    (Rendering|SetVisibility (Variables|Default|GetRifle_Player) false false)
    (Rendering|SetVisibility (Variables|Default|GetLauncher_Player) true false)))

(fn FireRifle
  (bind _rifle (Variables|Default|GetRifle))
  (bind _returnvalue (Transformation|GetSocketTransform _rifle "MuzzleFlashSocket" "RTS_World"))
  (Game|SpawnActorfromClass "/Game/BluePrint/Rifle_Projectile.Rifle_Projectile_C" _returnvalue "Undefined" 0 0)
  (Effects|Components|ParticleSystem|SetTemplate (Variables|Default|GetRifleMUzzleFlash) "/Game/SciFiWeapLight/FX/Particles/P_AssaultRifle_MuzzleFlash_Light.P_AssaultRifle_MuzzleFlash_Light")
  (Audio|PlaySoundatLocation "/Game/SciFiWeapLight/Sound/Rifle/Rifle_Fire_Cue.Rifle_Fire_Cue" (.Location (Math|Transform|BreakTransform _returnvalue)) "0, 0, 0" 1.0 1.0 0.0 0 0 0))

(fn FireLauncher
  (bind _launcher (Variables|Default|GetLauncher))
  (bind _returnvalue (Transformation|GetSocketTransform _launcher "MuzzleFlashSocket" "RTS_World"))
  (Utilities|FlowControl|DoOnce false
    (:Completed
      (Game|SpawnActorfromClass "/Game/BluePrint/Launcher_Projectile.Launcher_Projectile_C" _returnvalue "Undefined" 0 0)
      (Effects|Components|ParticleSystem|SetTemplate (Variables|Default|GetLauncherMuzzleFlash) "/Game/Effects/ParticleSystems/Weapons/RocketLauncher/Muzzle/P_Launcher_MF.P_Launcher_MF")
      (Audio|PlaySoundatLocation "/Game/Sounds/Weapons/GrenadeLauncher/SCue_Launcher_Shoot.SCue_Launcher_Shoot" (.Location (Math|Transform|BreakTransform _returnvalue)) "0, 0, 0" 1.0 1.0 0.0 0 0 0))))

(fn Sprint
  (Variables|Default|SetSprinting true)
  (Variables|/Script/Engine.CharacterMovementComponent|SetMaxWalkSpeed (Variables|Character|GetCharacterMovement) 8e+02))

(fn StopSprint
  (Variables|Default|SetSprinting false)
  (Variables|/Script/Engine.CharacterMovementComponent|SetMaxWalkSpeed (Variables|Character|GetCharacterMovement) 6e+02))

(fn ResetADS
  (if (and (Utilities|Enum|Equal(Enum) (Variables|Default|GetWeaponList) "NewEnumerator1") (Variables|Default|GetAiming))
    (CallFunction|Reset)))