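; PowerCube is a destructible cube actor with an Armor value, counted by the Shooter_GM game mode.
; Radial and any-damage events subtract from Armor and briefly swap the cube to a hit material as a flash.
; Tick polls Armor and destroys the actor at zero or below.
; On destruction it spawns a scaled-up explosion emitter and sound, then decrements the game mode's CurrentCube count.
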(event Game|Damage|EventRadialDamage
  (params (DamageReceived :type Float%20%28single-precision%29) (DamageType :type Damage%20Type%20Object%20Reference) (Origin :type Vector :default "0, 0, 0") (HitInfo :type Hit%20Result%20Structure%20%28by%20ref%29) (InstigatedBy :type Controller%20Object%20Reference) (DamageCauser :type Actor%20Object%20Reference))
  (bind _cube (Variables|Default|GetCube))
  ;[1 1 1] When Receiving Armor
  (Variables|Default|SetArmor (- (Variables|Default|GetArmor) DamageReceived))
  (Rendering|Material|SetMaterial _cube 0 "/Game/StarterContent/Materials/Hit_Material.Hit_Material")
  (Utilities|FlowControl|Delay 0.2)
  (Rendering|Material|SetMaterial _cube 0 "/Game/StarterContent/Materials/M_Tech_Hex_Tile.M_Tech_Hex_Tile"))

(event Game|Damage|EventAnyDamage
  (params (Damage :type Float%20%28single-precision%29) (DamageType :type Damage%20Type%20Object%20Reference) (InstigatedBy :type Controller%20Object%20Reference) (DamageCauser :type Actor%20Object%20Reference))
  (bind _cube (Variables|Default|GetCube))
  ;[1 1 1] When Receiving Armor
  (Variables|Default|SetArmor (- (Variables|Default|GetArmor) Damage))
  (Rendering|Material|SetMaterial _cube 0 "/Game/StarterContent/Materials/Hit_Material.Hit_Material")
  (Utilities|FlowControl|Delay 0.2)
  (Rendering|Material|SetMaterial _cube 0 "/Game/StarterContent/Materials/M_Tech_Hex_Tile.M_Tech_Hex_Tile"))

(event EventTick
  (params (DeltaSeconds :type Float%20%28single-precision%29))
  ;[1 1 1] Check the Armor of the Cube
  (CallFunction|DestroyCube))

(event EventDestroyed
  (bind _returnvalue (Game|GetGameMode))
  (bind _asshooter_gm (Utilities|Casting|CastToShooter_GM _returnvalue))
  ;[1 1 1] Once Cube is Destroyed
  (bind _returnvalue_2 (Effects|SpawnEmitteratLocation "/Game/StarterContent/Particles/P_Explosion.P_Explosion" (Transformation|GetActorLocation) (Transformation|GetActorRotation) "5.000000,5.000000,5.000000"))
  (Audio|SpawnSoundatLocation "/Game/StarterContent/Audio/Explosion_Cue.Explosion_Cue" (Transformation|GetWorldLocation _returnvalue_2) "0, 0, 0" 1.0 1.0 0.0 0 0)
  (Variables|/Game/BluePrint/Shooter_GM.Shooter_GM_C|SetCurrent%20Cube _asshooter_gm (- (Variables|/Game/BluePrint/Shooter_GM.Shooter_GM_C|GetCurrent%20Cube _asshooter_gm) 1)))

(fn ConstructionScript)

(fn DestroyCube
  ;[1 1 1] Does Cube Have Armor?
  (if (<= (Variables|Default|GetArmor) 0.0)
    (Actor|DestroyActor)))